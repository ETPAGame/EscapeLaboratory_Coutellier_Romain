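; BP_Body is the first-person player body, which adds the IMC_Movement mapping context on possession and handles Enhanced Input move and look.
; Interact runs a short debug-drawn sphere trace from the camera and checks hit actors for an interface, with no follow-up action yet.
; Overlapping actors receive a CheckIDMessage with a fixed ID, and construction calls AddAC0X00A21E.
; Legacy axis input events remain as empty stubs.
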(event Input|EnhancedActionEvents|EnhancedInputActionIA_Mouvement
  (params (ActionValue :type Vector%202D%20Structure) (ElapsedSeconds :type Float%20%28single-precision%29) (TriggeredSeconds :type Float%20%28single-precision%29))
  ;[0.006671 0.151 0] Controls
  (Pawn|Input|AddMovementInput (+ (* (.x ActionValue) (Transformation|GetActorForwardVector)) (* (.y ActionValue) (Transformation|GetActorRightVector))) 1.0 false))

(event Input|EnhancedActionEvents|EnhancedInputActionIA_Look
  (params (ActionValue :type Vector%202D%20Structure) (ElapsedSeconds :type Float%20%28single-precision%29) (TriggeredSeconds :type Float%20%28single-precision%29))
  ;[0.006671 0.151 0] HeadRotation
  (Pawn|Input|AddControllerYawInput (* (.x ActionValue) -1.0))
  (Pawn|Input|AddControllerPitchInput (.y ActionValue)))

(event Input|EnhancedActionEvents|EnhancedInputActionIA_Interact
  (params (ActionValue :type Boolean) (ElapsedSeconds :type Float%20%28single-precision%29) (TriggeredSeconds :type Float%20%28single-precision%29))
  (bind _firstpersoncamera (Variables|MyCharacter|GetFirstPersonCamera))
  (bind _returnvalue (Transformation|GetWorldLocation _firstpersoncamera))
  ;[0 0.3281 0] NeuralPsychicInteractionV2.0
  (bind _outhits (Collision|MultiSphereTraceByChannel _returnvalue (+ _returnvalue (* (Math|Vector|GetForwardVector _firstpersoncamera) 2e+02)) 1e+01 "TraceTypeQuery1" false 0 "ForDuration"))
  (bind _array_element (Utilities|Array|ForEachLoopwithBreak _outhits)
    (:LoopBody
      (if (Utilities|DoesObjectImplementInterface (.hitactor _array_element) 0)
        _))))

(event EventPossessed
  (params (NewController :type Controller%20Object%20Reference))
  ;[1 0 0] Initializing Neural connections
  (bind _asplayer_controller (Utilities|Casting|CastToPlayerController NewController))
  (Input|AddMappingContext (PlayerController|LocalPlayerSubsystems|GetEnhancedInputLocalPlayerSubsystem _asplayer_controller) "/Game/EurileneGene/Inputs/IMC_Movement.IMC_Movement" 0))

(event Collision|EventActorBeginOverlap
  (params (OtherActor :type Actor%20Object%20Reference))
  ;[1 0 0] ID
  (Class|BPIIdentity|CheckID(Message) OtherActor "id_29"))

(event Input|AxisEvents|InputAxisTurn
  (params (AxisValue :type Float%20%28single-precision%29))
  ;[0 0.3281 0] OLD
)

(event Input|AxisEvents|InputAxisLookUp
  (params (AxisValue :type Float%20%28single-precision%29))
  ;[0 0.3281 0] OLD
)

(event Input|AxisEvents|InputAxisMoveForward
  (params (AxisValue :type Float%20%28single-precision%29))
  ;[0 0.3281 0] OLD
)

(event Input|AxisEvents|InputAxisMoveRight
  (params (AxisValue :type Float%20%28single-precision%29))
  ;[0 0.3281 0] OLD
)

(fn ConstructionScript
  (Utilities|FlowControl|Sequence
    (:then_0
      (AddComponent|AddAC0X00A21E))
    (:then_1)))